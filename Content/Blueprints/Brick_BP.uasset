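; Brick actor that reacts to hits from Ball_BP and can be broken, as in a brick-breaker game.
; On BeginPlay it moves its Cube to a fixed height, keeping X and Y.
; When the ball overlaps BoxCollision, a brick with SecondHit set turns red and clears that flag.
; A brick without the flag destroys itself after a short delay, so flagged bricks take two hits.
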(event OnComponentBeginOverlap(BoxCollision)
  (params (OverlappedComponent :type Primitive%20Component%20Object%20Reference) (OtherActor :type Actor%20Object%20Reference) (OtherComp :type Primitive%20Component%20Object%20Reference) (OtherBodyIndex :type Integer) (bFromSweep :type Boolean) (SweepResult :type Hit%20Result%20Structure%20%28by%20ref%29))
  (Utilities|Casting|CastToBall_BP OtherActor)
  (if (Variables|Default|GetSecond%20Hit)
    (Rendering|Material|SetMaterial (Variables|Default|GetCube) 0 "/Game/Materials/Red.Red")
    (Variables|Default|SetSecond%20Hit false)
    (else
      (Utilities|FlowControl|Delay 0.2)
      (Actor|DestroyActor))))

(event EventBeginPlay
  (bind _cube (Variables|Default|GetCube))
  (bind _returnvalue (Transformation|GetWorldLocation _cube))
  (Transformation|SetWorldLocation (Variables|Default|GetCube) (Math|Vector|MakeVector (.x _returnvalue) (.y _returnvalue) 1e+02) false false))

(event Collision|EventActorBeginOverlap
  (params (OtherActor :type Actor%20Object%20Reference)))

(event EventTick
  (params (DeltaSeconds :type Float%20%28single-precision%29)))

(fn ConstructionScript)