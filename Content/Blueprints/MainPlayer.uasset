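; MainPlayer is a touch-controlled player Blueprint that slides its Player component along the world X axis to follow a finger.
; Touch press and release events set an IsTouching flag that Tick checks every frame.
; While touching, a Visibility trace under the first finger supplies X, while Y is kept and Z is fixed.
; Otherwise, Tick sets the root to its current location, leaving it in place.
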(event EventBeginPlay)

(event Collision|EventActorBeginOverlap
  (params (OtherActor :type Actor%20Object%20Reference)))

(event EventTick
  (params (DeltaSeconds :type Float%20%28single-precision%29))
  (bind _player (Variables|Default|GetPlayer))
  (bind _defaultsceneroot (Variables|Default|GetDefaultSceneRoot))
  ;[1 1 1] If Finger is On Screen
  (if (Variables|Default|GetIsTouching)
    (Transformation|SetWorldLocation _player (Math|Vector|MakeVector (.X (Math|Vector|BreakVector (.location (.HitResult (Class|PlayerController|GetHitResultUnderFingerbyChannel (Game|GetPlayerController 0) "Touch1" "TraceTypeQuery1" true))))) (.y (Transformation|GetWorldLocation _player)) 1e+02) false false)
    (else
      ;[1 1 1] If Finger is not On Screen
      (Transformation|SetWorldLocation _defaultsceneroot (Transformation|GetWorldLocation _defaultsceneroot) false false))))

(event Input|TouchEvents|InputTouch
  (params (Location :type Vector) (FingerIndex :type ETouchIndex%20Enum))
  (:Pressed
    (Variables|Default|SetIsTouching true))
  (:Released
    (Variables|Default|SetIsTouching false)))

(fn ConstructionScript)